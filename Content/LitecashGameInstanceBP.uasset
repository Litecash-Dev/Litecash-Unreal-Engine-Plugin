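; Game instance Blueprint that manages the lifecycle of Litecash services (node, explorer node, wallet and wallet API) alongside the game.
; On Init it starts each service enabled by its Run flag, in that order, and stores the returned state.
; On Shutdown it stops whichever services are running in reverse order, updating each state variable.
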(event `self.ReceiveInit`
  (`self.InitLitecash`))

(event `self.ReceiveShutdown`
  (`self.ShutdownLitecash`))

(fn `InitLitecash`
  (`|ExecutionSequence`
    (:`then_0`
      (if (`self.RunNode`)
        (bind _returnvalue (`self.StartNode`))
        (set `self.NodeState` _returnvalue)))
    (:`then_1`
      (if (`self.RunExplorerNode`)
        (bind _returnvalue_2 (`self.StartExplorerNode`))
        (set `self.ExplorerNodeState` _returnvalue_2)))
    (:`then_2`
      (if (`self.RunWallet`)
        (bind _returnvalue_3 (`self.StartWallet`))
        (set `self.WalletState` _returnvalue_3)))
    (:`then_3`
      (if (`self.RunWalletAPI`)
        (bind _returnvalue_4 (`self.StartWalletAPI`))
        (set `self.WalletAPIState` _returnvalue_4)))))

(fn `ShutdownLitecash`
  (`|ExecutionSequence`
    (:`then_0`
      (if (`self.IsWalletAPIRunning`)
        (bind _returnvalue (`self.StopWalletAPI`))
        (set `self.WalletAPIState` _returnvalue)))
    (:`then_1`
      (if (`self.IsWalletRunning`)
        (bind _returnvalue_2 (`self.StopWallet`))
        (set `self.WalletState` _returnvalue_2)))
    (:`then_2`
      (if (`self.IsExplorerNodeRunning`)
        (bind _returnvalue_3 (`self.StopExplorerNode`))
        (set `self.ExplorerNodeState` _returnvalue_3)))
    (:`then_3`
      (if (`self.IsNodeRunning`)
        (bind _returnvalue_4 (`self.StopNode`))
        (set `self.NodeState` _returnvalue_4)))))